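; ProgressFeed_BP is a pickup that advances level progress when the player pawn overlaps it.
; On overlap with Player0CharacterPawn_BP, it adds a fixed amount to CurrentProgress on the game state, calls CheckProgress, then destroys itself.
; It casts to Player0_GameStateBase_BP first and falls back to ProceduralLevel1_GSB, supporting both game state classes.
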(event `self.ReceiveActorBeginOverlap`
  (params (OtherActor :type "Actor Object Reference"))
  (bind _returnvalue (`GameplayStatics.GetGameState`))
  (cast `/Game/Players/Player0/Player0CharacterPawn_BP` OtherActor)
  (bind _asplayer_0_game_state_base_bp (cast `/Game/Players/Player0/Player0_GameStateBase_BP` _returnvalue)
    (:`then`
      (set `/Game/Players/Player0/Player0_GameStateBase_BP.Current Progress` (+ (`/Game/Players/Player0/Player0_GameStateBase_BP.Current Progress` _asplayer_0_game_state_base_bp) 10.0) _asplayer_0_game_state_base_bp)
      (`/Game/Players/Player0/Player0_GameStateBase_BP.CheckProgress` _asplayer_0_game_state_base_bp)
      (`self.K2_DestroyActor`))
    (:`CastFailed`
      (bind _asprocedural_level_1_gsb (cast `/Game/Levels/ProceduralLevel1/ProceduralLevel1_GSB` _returnvalue))
      (set `/Game/Levels/ProceduralLevel1/ProceduralLevel1_GSB.Current Progress` (+ (`/Game/Levels/ProceduralLevel1/ProceduralLevel1_GSB.Current Progress` _asprocedural_level_1_gsb) 10.0) _asprocedural_level_1_gsb)
      (`/Game/Levels/ProceduralLevel1/ProceduralLevel1_GSB.CheckProgress` _asprocedural_level_1_gsb)
      (`self.K2_DestroyActor`))))

(fn `UserConstructionScript`)