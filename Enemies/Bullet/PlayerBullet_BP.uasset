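; Player bullet actor that damages enemies through overlap and moves with a ProjectileMovement component.
; On overlap it ignores actors tagged Player, applies fixed damage to those tagged Enemy, and destroys itself on any non-player contact.
; A server-to-multicast event pair, named for networked movement, sets the projectile's local-space velocity, but its only call in this graph is unreachable.
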(event `self.ReceiveBeginPlay`
  ;[1 1 1] Begin Play
)

(event `self.ReceiveActorBeginOverlap`
  (params (OtherActor :type "Actor Object Reference"))
  ;[1 1 1] Event BeginOverlap
  (if (not (`self.ActorHasTag` OtherActor "Player"))
    (if (`self.ActorHasTag` OtherActor "Enemy")
      (`GameplayStatics.ApplyDamage` OtherActor 2.0))
    (`self.K2_DestroyActor`)))

(event `ServerMoveToTarget`
  (params (Velocity :type "Vector Structure"))
  ;[1 1 1] Networked Bullet Movement
  (`self.MulticastMoveToTarget` (`self.Velocity`)))

(event `MulticastMoveToTarget`
  (params (Velocity :type "Vector Structure"))
  (bind _projectilemovement (`self.ProjectileMovement`))
  ;[1 1 1] Networked Bullet Movement
  (`/Engine/EditorBlueprintResources/StandardMacros.IsValid` _projectilemovement
    (:`Is Valid`
      (`ProjectileMovementComponent.SetVelocityInLocalSpace` _projectilemovement Velocity))))

(fn `UserConstructionScript`)