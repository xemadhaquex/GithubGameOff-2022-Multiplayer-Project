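; Enemy bullet projectile that damages the player pawn on overlap and destroys itself after overlapping any actor.
; Movement and destruction go through Server events that call Multicast events for networking.
; The move event ignores its Destination, setting a fixed local forward velocity on ProjectileMovement.
; An AI MoveTo call and a filter sparing enemies and other bullets are left disconnected.
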(event `self.ReceiveActorBeginOverlap`
  (params (OtherActor :type "Actor Object Reference"))
  ;[1 1 1] On Overlap
  (bind _asplayer_0character_pawn_bp (cast `/Game/Players/Player0/Player0CharacterPawn_BP` OtherActor)
    (:`then`
      (`GameplayStatics.ApplyDamage` _asplayer_0character_pawn_bp 20.0))
    (:`CastFailed`
      _))
  (`self.Server Destroy`))

(event `Server Destroy`
  ;[1 1 1] Destroy Bullet
  (`self.MulticastDestroy`))

(event `ServerMoveToTarget`
  (params (Destination :type "Vector Structure"))
  ;[1 1 1] Networked Projectile Movement
  (`self.MulticastMoveToTarget` Destination))

(event `MulticastDestroy`
  ;[1 1 1] Destroy Bullet
  (`self.K2_DestroyActor`))

(event `MulticastMoveToTarget`
  (params (Destination :type "Vector Structure"))
  ;[1 1 1] Networked Projectile Movement
  (`ProjectileMovementComponent.SetVelocityInLocalSpace` (`self.ProjectileMovement`) (600.0 0.0 0.0)))

(fn `UserConstructionScript`)